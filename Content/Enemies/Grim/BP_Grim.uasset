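; Grim is a ranged AI enemy that detects the player, closes in and fires light or heavy projectiles.
; A trigger overlap or PawnSensing calls FollowPlayer, which moves within range and randomly plays one of two attack montages, favoring the first.
; CanAttack gates this until the montage ends.
; LightAttack and HeavyAttack events, not called within this graph, turn Grim toward the player and spawn projectiles from their arrow components.
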(event `FollowPlayer`
  ;[0.06274 0.06274 0.06274 1 25] AI_Enemy
  ;;[0 0.006563 0.04688] Moving to Player
  (if (`self.CanAttack?`)
    (set `self.CanAttack?` false)
    (if (`self.IsSeeingPlayer?`)
      (`|AIMoveTo` self (0.0 0.0 0.0) (`GameplayStatics.GetPlayerCharacter` 0) 2000.0
        (:`OnSuccess`
          ;;[0.08333 0 0] Attack Selection
          (set `MovementComponent.Velocity` (0.0 0.0 0.0) (`self.CharacterMovement`))
          (switch `int` (`KismetMathLibrary.RandomIntegerInRange` 1 3)
            (:`1`
              (bind _returnvalue (`self.PlayAnimMontage` "/Game/Enemies/Grim/Attack1_AnimMontage.Attack1_AnimMontage" :!label _label))
              (`KismetSystemLibrary.Delay` _returnvalue)
              (set `self.CanAttack?` true))
            (:`2`
              (goto _label))
            (:`3`
              (bind _returnvalue_2 (`self.PlayAnimMontage` "/Game/Enemies/Grim/Attack2_AnimMontage.Attack2_AnimMontage"))
              (`KismetSystemLibrary.Delay` _returnvalue_2)
              (set `self.CanAttack?` true))))))))

(event `self.TrackTrigger.OnComponentBeginOverlap`
  (params (OverlappedComponent :type "PrimitiveComponent Object Reference") (OtherActor :type "Actor Object Reference") (OtherComp :type "PrimitiveComponent Object Reference") (OtherBodyIndex :type Integer) (bFromSweep :type Boolean) (SweepResult :type "HitResult Structure (by ref)"))
  ;[0.06274 0.06274 0.06274 1 25] AI_Enemy
  ;;[0.001063 0.04167 0] Detection Player
  (if (== OtherActor (`GameplayStatics.GetPlayerCharacter` 0))
    (set `self.IsSeeingPlayer?` true :!label _label_2)
    (`self.FollowPlayer`)))

(event `self.PawnSensing.OnSeePawn`
  (params (Pawn :type "Pawn Object Reference"))
  ;[0.06274 0.06274 0.06274 1 25] AI_Enemy
  ;;[0.001063 0.04167 0] Detection Player
  (if (== (stale `self.TrackTrigger.OnComponentBeginOverlap` OtherActor) (`GameplayStatics.GetPlayerCharacter` 0))
    (goto _label_2)))

(event `LightAttack`
  ;[0.06274 0.06274 0.06274] Light Attack
  (`self.K2_SetActorRotation` (`KismetMathLibrary.FindLookAtRotation` (`SceneComponent.K2_GetComponentLocation` (`self.CapsuleComponent`)) (`self.K2_GetActorLocation` (`GameplayStatics.GetPlayerPawn` 0))))
  (`|SpawnActorFromClass` "/Game/Enemies/Grim/BP_LightProjectile_Grim.BP_LightProjectile_Grim_C" (`SceneComponent.K2_GetComponentToWorld` (`self.ArrowLight`)) "AlwaysSpawn" "MultiplyWithRoot" null null))

(event `HeavyAttack`
  ;[0.06274 0.06274 0.06274] Heavy Attack
  (`self.K2_SetActorRotation` (`KismetMathLibrary.FindLookAtRotation` (`SceneComponent.K2_GetComponentLocation` (`self.CapsuleComponent`)) (`self.K2_GetActorLocation` (`GameplayStatics.GetPlayerPawn` 0))))
  (`|SpawnActorFromClass` "/Game/Enemies/Grim/BP_HeavyProjectile_Grim.BP_HeavyProjectile_Grim_C" (`SceneComponent.K2_GetComponentToWorld` (`self.ArrowHeavy`)) "AlwaysSpawn" "MultiplyWithRoot" null null))

(fn `UserConstructionScript`)