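; Enemy AI Blueprint that moves toward the player character and performs a melee-style montage attack on arrival.
; A TrackTrigger overlap or PawnSensing sighting sets IsSeeingPlayer and calls FollowPlayer, which runs AIMoveTo toward the player.
; On a successful move, it zeroes velocity and plays the attack montage, using CanAttack and a montage-length Delay as a cooldown.
; FollowPlayer does not loop, so each chase starts from a trigger event.
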(event `self.TrackTrigger.OnComponentBeginOverlap`
  (params (OverlappedComponent :type "PrimitiveComponent Object Reference") (OtherActor :type "Actor Object Reference") (OtherComp :type "PrimitiveComponent Object Reference") (OtherBodyIndex :type Integer) (bFromSweep :type Boolean) (SweepResult :type "HitResult Structure (by ref)"))
  (set `self.IsSeeingPlayer?` true :!label _label)
  (`self.FollowPlayer`))

(event `self.PawnSensing.OnSeePawn`
  (params (Pawn :type "Pawn Object Reference"))
  (goto _label))

(event `FollowPlayer`
  (if (`self.IsSeeingPlayer?`)
    (`|AIMoveTo` self (0.0 0.0 0.0) (`GameplayStatics.GetPlayerCharacter` 0) 300.0
      (:`OnSuccess`
        (if (`self.CanAttack?`)
          (set `self.CanAttack?` false)
          (set `MovementComponent.Velocity` (0.0 0.0 0.0) (`self.CharacterMovement`))
          (bind _returnvalue (`self.PlayAnimMontage` "/Game/Enemies/Crunch/Attack1_AnimMontage.Attack1_AnimMontage"))
          (`KismetSystemLibrary.Delay` _returnvalue)
          (set `self.CanAttack?` true))))))

(fn `UserConstructionScript`)