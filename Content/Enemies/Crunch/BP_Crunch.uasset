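; Crunch enemy AI that chases the player once seen or inside its track trigger, then attacks with melee montages.
; A CanAttack-gated move picks the light attack two times in three, otherwise the heavy, re-arming after the montage's length.
; AttackStart/AttackEnd toggle hit-box collision; overlaps call Damage behind one-second DoOnce cooldowns.
; Damage sets player health to damage minus current health, a reversed subtraction.
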(event `FollowPlayer`
  ;[0.06274 0.06274 0.06274 1 25] AI_Enemy
  ;;[0 0.006563 0.04688] Moving to Player
  (if (`self.CanAttack?`)
    (set `self.CanAttack?` false)
    (if (`self.IsSeeingPlayer?`)
      (`|AIMoveTo` self (0.0 0.0 0.0) (`GameplayStatics.GetPlayerCharacter` 0) 200.0 true
        (:`OnSuccess`
          ;;[0.08333 0 0] Attack Selection
          (set `MovementComponent.Velocity` (0.0 0.0 0.0) (`self.CharacterMovement`))
          (switch `int` (`KismetMathLibrary.RandomIntegerInRange` 1 3)
            (:`1`
              (bind _returnvalue (`self.PlayAnimMontage` "/Game/Enemies/Crunch/Attack1_AnimMontage.Attack1_AnimMontage" :!label _label))
              (`KismetSystemLibrary.Delay` _returnvalue)
              (set `self.CanAttack?` true))
            (:`2`
              (goto _label))
            (:`3`
              (bind _returnvalue_2 (`self.PlayAnimMontage` "/Game/Enemies/Crunch/Attack2_AnimMontage.Attack2_AnimMontage"))
              (`KismetSystemLibrary.Delay` _returnvalue_2)
              (set `self.CanAttack?` true))))))))

(event `self.PawnSensing.OnSeePawn`
  (params (Pawn :type "Pawn Object Reference"))
  ;[0.06274 0.06274 0.06274 1 25] AI_Enemy
  ;;[0.001063 0.04167 0] Detection Player
  (set `self.IsSeeingPlayer?` true :!label _label_2)
  (`self.FollowPlayer`))

(event `self.TrackTrigger.OnComponentBeginOverlap`
  (params (OverlappedComponent :type "PrimitiveComponent Object Reference") (OtherActor :type "Actor Object Reference") (OtherComp :type "PrimitiveComponent Object Reference") (OtherBodyIndex :type Integer) (bFromSweep :type Boolean) (SweepResult :type "HitResult Structure (by ref)"))
  ;[0.06274 0.06274 0.06274 1 25] AI_Enemy
  ;;[0.001063 0.04167 0] Detection Player
  (goto _label_2))

(event `self.Attack1_Collision.OnComponentBeginOverlap`
  (params (OverlappedComponent :type "PrimitiveComponent Object Reference") (OtherActor :type "Actor Object Reference") (OtherComp :type "PrimitiveComponent Object Reference") (OtherBodyIndex :type Integer) (bFromSweep :type Boolean) (SweepResult :type "HitResult Structure (by ref)"))
  ;[0.06274 0.06274 0.06274 1 25] Attacks
  ;;[0.06274 0.06274 0.06274] Light Attack
  (`/Engine/EditorBlueprintResources/StandardMacros.DoOnce` false :!label _label_3
    (:`Completed`
      (`self.Damage` 10.0)
      (`KismetSystemLibrary.PrintString` "OUUUCH")
      (`KismetSystemLibrary.Delay` 1.0)
      (goto _label_3 :!via `Reset`))))

(event `self.Attack2_Collision.OnComponentBeginOverlap`
  (params (OverlappedComponent :type "PrimitiveComponent Object Reference") (OtherActor :type "Actor Object Reference") (OtherComp :type "PrimitiveComponent Object Reference") (OtherBodyIndex :type Integer) (bFromSweep :type Boolean) (SweepResult :type "HitResult Structure (by ref)"))
  ;[0.06274 0.06274 0.06274 1 25] Attacks
  ;;[0.06274 0.06274 0.06274] Heavy Attack
  (`/Engine/EditorBlueprintResources/StandardMacros.DoOnce` false :!label _label_4
    (:`Completed`
      (`self.Damage` 20.0)
      (`KismetSystemLibrary.PrintString` "AÏEUUUUUUUUUU")
      (`KismetSystemLibrary.Delay` 1.0)
      (goto _label_4 :!via `Reset`))))

(event `self.ReceiveBeginPlay`
  (`PrimitiveComponent.SetCollisionEnabled` (`self.Attack1_Collision`) "NoCollision")
  (`PrimitiveComponent.SetCollisionEnabled` (`self.Attack2_Collision`) "NoCollision"))

(fn `AttackEnd`
  (params (`Collision box Ref` :type "PrimitiveComponent Object Reference"))
  (`PrimitiveComponent.SetCollisionEnabled` `Collision box Ref` "NoCollision"))

(fn `AttackStart`
  (params (`Box Collision Ref` :type "PrimitiveComponent Object Reference"))
  (`PrimitiveComponent.SetCollisionEnabled` `Box Collision Ref` "QueryAndPhysics"))

(fn `Damage`
  (params (Damage :type "Float (double-precision)"))
  (bind _asbp_third_person_character (cast `/Game/ThirdPerson/Blueprints/BP_ThirdPersonCharacter` (`GameplayStatics.GetPlayerCharacter` 0)))
  (set `/Game/ThirdPerson/Blueprints/BP_ThirdPersonCharacter.CurrentHealth` (- Damage (`/Game/ThirdPerson/Blueprints/BP_ThirdPersonCharacter.CurrentHealth` _asbp_third_person_character)) _asbp_third_person_character)
  (return))

(fn `UserConstructionScript`)