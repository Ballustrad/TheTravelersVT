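; BP_HeavyProjectile_Grim is a heavy projectile for the Grim enemy, meant to hurt the player on hit.
; On a ProjectileCollision hit it compares HitComponent, rather than the other actor, to the player pawn, calls Damage on a match, and destroys itself either way.
; Damage ignores its amount input and negates BP_ThirdPersonCharacter's CurrentHealth instead of subtracting.
; Overlap and hit events also print debug strings.
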(event `self.ProjectileCollision.OnComponentBeginOverlap`
  (params (OverlappedComponent :type "PrimitiveComponent Object Reference") (OtherActor :type "Actor Object Reference") (OtherComp :type "PrimitiveComponent Object Reference") (OtherBodyIndex :type Integer) (bFromSweep :type Boolean) (SweepResult :type "HitResult Structure (by ref)"))
  (`KismetSystemLibrary.PrintString` "Hello"))

(event `self.ProjectileCollision.OnComponentHit`
  (params (HitComponent :type "PrimitiveComponent Object Reference") (OtherActor :type "Actor Object Reference") (OtherComp :type "PrimitiveComponent Object Reference") (NormalImpulse :type "Vector Structure") (Hit :type "HitResult Structure (by ref)"))
  (`KismetSystemLibrary.PrintString` "Hello")
  (if (== HitComponent (`GameplayStatics.GetPlayerPawn` 0))
    (`self.Damage` 10.0)
    (`KismetSystemLibrary.PrintString` "OUUUCH")
    (`self.K2_DestroyActor`)
    (else
      (`self.K2_DestroyActor`))))

(fn `Damage`
  (params (Damage :type "Float (double-precision)"))
  (bind _asbp_third_person_character (cast `/Game/ThirdPerson/Blueprints/BP_ThirdPersonCharacter` (`GameplayStatics.GetPlayerCharacter` 0)))
  (set `/Game/ThirdPerson/Blueprints/BP_ThirdPersonCharacter.CurrentHealth` (- 0.0 (`/Game/ThirdPerson/Blueprints/BP_ThirdPersonCharacter.CurrentHealth` _asbp_third_person_character)) _asbp_third_person_character)
  (return))

(fn `UserConstructionScript`)